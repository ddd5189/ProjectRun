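; BP_StartEndLine is a trigger line actor that starts or ends a timed level run when the player crosses it.
; On overlap, a player check returns the character and branches on TimerStarted in the linked Other actor.
; If unset, it starts the character's timer and flags itself; if set, it resets the timer, shows EndLevelWidget and pauses.
; ShowTimer forwards timer visibility to PlayerHUD.
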(event `self.ReceiveActorBeginOverlap`
  (params (OtherActor :type "Actor Object Reference"))
  (bind (_yes_no _character) (message `/Game/Actors(BP)/Interfaces/BPI_Player.IsPlayer` OtherActor))
  (if _yes_no
    (if (`/Game/Actors(BP)/BP_StartEndLine.TimerStarted` (`self.Other`))
      (`/Game/ThirdPersonBP/Blueprints/ThirdPersonCharacter.ResetTimer` _character true)
      (bind _output_get (set `/Game/Actors(BP)/BP_StartEndLine.TimerStarted` false (`self.Other`)))
      (`self.ShowTimer` _output_get)
      (bind _returnvalue (`|CreateWidget` "/Game/Actors(BP)/Widgets/EndLevelWidget.EndLevelWidget_C"))
      (bind _output_get_2 (set `self.EndWidget` _returnvalue))
      (`UserWidget.AddToViewport` _output_get_2 0)
      (`GameplayStatics.SetGamePaused` true)
      (else
        (`/Game/ThirdPersonBP/Blueprints/ThirdPersonCharacter.StartTimer` _character)
        (bind _output_get_3 (set `self.TimerStarted` true))
        (`self.ShowTimer` _output_get_3)))))

(fn `ShowTimer`
  (params (`True/False` :type Boolean))
  (bind _asplayer_hud (cast `/Game/ThirdPersonBP/Blueprints/HUD/PlayerHUD` (`PlayerController.GetHUD` (`GameplayStatics.GetPlayerController` 0))))
  (`/Game/ThirdPersonBP/Blueprints/HUD/PlayerHUD.ShowTimer` _asplayer_hud `True/False`))

(fn `UserConstructionScript`)